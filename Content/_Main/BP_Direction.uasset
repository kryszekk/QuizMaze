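; BP_Direction is a clickable direction arrow that sends the player to its target crossroads.
; A mesh click or ClickonDirection call passes TargetCrossroads to the player controller through MoveToCrossroadsMessage, printing an error if unset.
; Hovering plays a sound, spawns an effect at the target and runs a looping timer that pulses the mesh scale until the cursor leaves.
; The construction script optionally yaws the arrow toward its target.
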(event `self.ReceiveBeginPlay`
  (set `self.InitialScale` (`SceneComponent.RelativeScale3D` (`self.StaticMesh`))))

(event `/Game/_Main/BI_Direction.ClickOnDirection`
  (`/Engine/EditorBlueprintResources/StandardMacros.IsValid` (`self.TargetCrossroads`) :!label _label
    (:`Is Valid`
      ;[0 0.000581 0.005] Move to the new crossroads
      (message `/Game/_Main/BI_TopDownController.MoveToCrossroads` (`GameplayStatics.GetPlayerController` 0) (`self.TargetCrossroads`)))
    (:`Is Not Valid`
      (`KismetSystemLibrary.PrintString` (`KismetStringLibrary.Concat_StrStr` "Error: \n" "Direction arrow doesnt have a Target crossroads set \n" (`KismetSystemLibrary.GetDisplayName` self))))))

(event `self.StaticMesh.OnClicked`
  (params (TouchedComponent :type "PrimitiveComponent Object Reference") (ButtonPressed :type "Key Structure"))
  (goto _label))

(event `self.StaticMesh.OnBeginCursorOver`
  (params (TouchedComponent :type "PrimitiveComponent Object Reference"))
  (bind _initialscale_x (`KismetMathLibrary.BreakVector` (`self.InitialScale`)))
  (`GameplayStatics.PlaySound2D` "/Engine/VREditor/Sounds/UI/Gizmo_Handle_Clicked.Gizmo_Handle_Clicked" 1.0 1.0 0.0 null null)
  (`NiagaraFunctionLibrary.SpawnSystemAtLocation` (`self.FXCursor`) (`self.K2_GetActorLocation` (`self.TargetCrossroads`)))
  (bind _returnvalue (`KismetSystemLibrary.K2_SetTimerDelegate` (delegate `Tick`) 0.01 true))
  (set `self.ScaleHande` _returnvalue)
  (set `self.InterpTo` (* _initialscale_x 1.5)))

(event `Tick`
  (bind _initialscale_x (`KismetMathLibrary.BreakVector` (`self.InitialScale`)))
  (bind _initialscale_x_2 (`KismetMathLibrary.BreakVector` (`self.InitialScale`)))
  (bind _relativescale3d_x (`KismetMathLibrary.BreakVector` (`SceneComponent.RelativeScale3D` (`self.StaticMesh`))))
  (bind _relativescale3d_x_2 (`KismetMathLibrary.BreakVector` (`SceneComponent.RelativeScale3D` (`self.StaticMesh`))))
  (bind _returnvalue (`KismetMathLibrary.FInterpTo` _relativescale3d_x_2 (`self.InterpTo`) (`GameplayStatics.GetWorldDeltaSeconds`) 2.4))
  ;[0 0.000581 0.005] Do interp to
  (`SceneComponent.SetRelativeScale3D` (`self.StaticMesh`) (`KismetMathLibrary.MakeVector` _returnvalue _returnvalue _returnvalue))
  (if (`KismetMathLibrary.NearlyEqual_FloatFloat` (`self.InterpTo`) _relativescale3d_x 0.1)
    (`/Engine/EditorBlueprintResources/StandardMacros.FlipFlop`
      (:`A`
        (set `self.InterpTo` _initialscale_x_2))
      (:`B`
        (set `self.InterpTo` (* _initialscale_x (`self.ScaleTarget`)))))))

(event `self.StaticMesh.OnEndCursorOver`
  (params (TouchedComponent :type "PrimitiveComponent Object Reference"))
  (`KismetSystemLibrary.K2_ClearAndInvalidateTimerHandle` (`self.ScaleHande`))
  (`SceneComponent.SetRelativeScale3D` (`self.StaticMesh`) (`self.InitialScale`)))

(fn `AutoRotate`
  (bind (_returnvalue_roll _returnvalue_pitch _returnvalue_yaw) (`KismetMathLibrary.BreakRotator` (`KismetMathLibrary.FindLookAtRotation` (`self.K2_GetActorLocation`) (`self.K2_GetActorLocation` (`self.TargetCrossroads`)))))
  (if (`self.bAutoRotate`)
    (`self.K2_SetActorRotation` (`KismetMathLibrary.MakeRotator` 0.0 0.0 _returnvalue_yaw))))

(fn `NewFunction`
  (params (InterpTo :type "Vector Structure"))
  (returns (bDirection :type Boolean))
  (`|ExecutionSequence`))

(fn `UserConstructionScript`
  (`self.AutoRotate`))