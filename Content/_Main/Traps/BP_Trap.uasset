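; BP_Trap is a base trap Blueprint whose logic ticks only while a player is nearby.
; BeginPlay starts a fast looping timer with a randomized initial delay, then pauses it shortly afterward.
; ActivateArea overlaps with actors tagged "Player" unpause the timer on entry and pause it on exit.
; Each timer firing calls OnTrapTick, an empty function that serves as the hook for trap behavior.
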(event `self.ReceiveBeginPlay`
  ;[0 0.000581 0.005] Traps are meant to work only if player is nearby
  (bind _returnvalue (`KismetSystemLibrary.K2_SetTimerDelegate` (delegate `TrapTick`) 0.1 true 0.2 0.2))
  (set `self.TimerHandle` _returnvalue)
  (`KismetSystemLibrary.Delay` 0.3)
  (`KismetSystemLibrary.K2_PauseTimerHandle` (`self.TimerHandle`)))

(event `self.ActivateArea.OnComponentBeginOverlap`
  (params (OverlappedComponent :type "PrimitiveComponent Object Reference") (OtherActor :type "Actor Object Reference") (OtherComp :type "PrimitiveComponent Object Reference") (OtherBodyIndex :type Integer) (bFromSweep :type Boolean) (SweepResult :type "HitResult Structure (by ref)"))
  (if (`self.ActorHasTag` OtherActor "Player")
    ;[0 0.000581 0.005] Traps are meant to work only if player is nearby
    (`KismetSystemLibrary.K2_UnPauseTimerHandle` (`self.TimerHandle`))))

(event `self.ActivateArea.OnComponentEndOverlap`
  (params (OverlappedComponent :type "PrimitiveComponent Object Reference") (OtherActor :type "Actor Object Reference") (OtherComp :type "PrimitiveComponent Object Reference") (OtherBodyIndex :type Integer))
  (if (`self.ActorHasTag` OtherActor "Player")
    ;[0 0.000581 0.005] Traps are meant to work only if player is nearby
    (`KismetSystemLibrary.K2_PauseTimerHandle` (`self.TimerHandle`))))

(event `TrapTick`
  ;[0 0.000581 0.005] Traps are meant to work only if player is nearby
  (`self.OnTrapTick`))

(fn `OnTrapTick`
  (return))

(fn `UserConstructionScript`)