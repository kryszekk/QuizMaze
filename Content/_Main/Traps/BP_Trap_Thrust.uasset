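; BP_Trap_Thrust is a trap Blueprint that pushes its static mesh along the actor's forward vector.
; On each parent-driven trap tick, an interpolated value eases toward its target and flips between Distance and zero on arrival.
; That value is added to the mesh's current relative location with a swept move, so it acts as a cumulative per-tick step rather than an absolute offset.
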(event `self.ReceiveBeginPlay`
  (`parent.ReceiveBeginPlay`))

(fn `OnTrapTick`
  (locals (NewLocalVar :type Boolean :default true))
  (bind _staticmesh (`self.StaticMesh`))
  (`parent.OnTrapTick`)
  ;[1 1 1] Move mesh
  (set `self.Current` (`KismetMathLibrary.FInterpTo` (`self.Current`) (`self.Target`) (`GameplayStatics.GetWorldDeltaSeconds`) 5.0))
  (`SceneComponent.K2_SetRelativeLocation` _staticmesh (+ (`SceneComponent.RelativeLocation` _staticmesh) (* (`self.GetActorForwardVector`) (`self.Current`))) true false)
  (if (`KismetMathLibrary.NearlyEqual_FloatFloat` (`self.Current`) (`self.Target`) 1.0)
    ;[1 1 1] Direction control
    (set `self.bForward` (not (`self.bForward`)))
    (if (`self.bForward`)
      (set `self.Target` (`self.Distance`))
      (else
        (set `self.Target` 0.0)))))

(fn `UserConstructionScript`
  (`parent.UserConstructionScript`))