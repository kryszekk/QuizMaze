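; BP_Crossroads is a crossroads actor that shows and hides the direction actors placed around it.
; On BeginPlay it box-traces through the HookUpDIrections volume for WorldDynamic components tagged "Direction", stores their actors and hides them.
; Trigger and BISetDirectionsVisibility events toggle those actors' static meshes, switching visibility and collision together.
; GetDirections exposes the stored list; the overlap events and ReferenceDIrections are inactive.
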(event `self.ReceiveBeginPlay`
  (bind _directions (`self.LookForDirections`))
  (set `self.Directions` _directions)
  ;[0 0.000581 0.005] Initialy all directions are hidden
  (`self.SetDirectionsVisibility` false))

(event `/Game/_Main/BI_Crossroads.BI_SetDirectionsVisibility`
  (params (bNewVisibility :type Boolean))
  (`self.SetDirectionsVisibility` bNewVisibility))

(event `Trigger`
  (params (bState :type Boolean))
  (`self.SetDirectionsVisibility` bState))

(event `self.Box.OnComponentBeginOverlap`
  (params (OverlappedComponent :type "PrimitiveComponent Object Reference") (OtherActor :type "Actor Object Reference") (OtherComp :type "PrimitiveComponent Object Reference") (OtherBodyIndex :type Integer) (bFromSweep :type Boolean) (SweepResult :type "HitResult Structure (by ref)")))

(event `self.Box.OnComponentEndOverlap`
  (params (OverlappedComponent :type "PrimitiveComponent Object Reference") (OtherActor :type "Actor Object Reference") (OtherComp :type "PrimitiveComponent Object Reference") (OtherBodyIndex :type Integer)))

(fn `GetDirections`
  (returns (Directions :type "Array of Actor Object Reference"))
  (return (`self.Directions`)))

(fn `LookForDirections`
  (returns (Directions :type "Array of Actor Object Reference"))
  (locals (DirectionsLocal :type "Array of Actor Object Reference"))
  (bind _hookupdirections (`self.HookUpDIrections`))
  (bind _returnvalue (`BoxComponent.GetScaledBoxExtent` _hookupdirections))
  (bind _returnvalue_2 (`SceneComponent.K2_GetComponentLocation` _hookupdirections))
  (bind _returnvalue_3 (`SceneComponent.GetForwardVector` _hookupdirections))
  (bind _returnvalue_4 (`KismetSystemLibrary.MakeLiteralDouble` (.x _returnvalue)))
  (bind (_outhits _returnvalue_5) (`KismetSystemLibrary.BoxTraceMultiForObjects` :`Start` (+ _returnvalue_2 (* _returnvalue_3 _returnvalue_4)) :`End` (+ _returnvalue_2 (* (`KismetMathLibrary.NegateVector` _returnvalue_3) _returnvalue_4)) :`HalfSize` (`KismetMathLibrary.MakeVector` 0.0 (.y _returnvalue) (.z _returnvalue)) :`ObjectTypes` (`|MakeArray` "ObjectTypeQuery2" :!type "EObjectTypeQuery Enum") :`bTraceComplex` true :`DrawTime` 1.0))
  (if _returnvalue_5
    (for _array_element _outhits
      (bind (_bblockinghit _binitialoverlap _time _distance _location _impactpoint _normal _impactnormal _physmat _hitactor _hitcomponent) (`GameplayStatics.BreakHitResult` _array_element))
      (if (`ActorComponent.ComponentHasTag` _hitcomponent "Direction")
        (`KismetArrayLibrary.Array_Add` (`local.DirectionsLocal`) _hitactor)))
    (return (`local.DirectionsLocal`))))

(fn `ReferenceDIrections`)

(fn `SetDirectionsVisibility`
  (params (bNewVisibility :type Boolean))
  (locals (bNewVisibilityLocal :type Boolean))
  (set `local.bNewVisibilityLocal` bNewVisibility)
  (for _array_element (`self.Directions`)
    (for _array_element_2 (`self.K2_GetComponentsByClass` _array_element "/Script/Engine.StaticMeshComponent")
      (`SceneComponent.SetVisibility` _array_element_2 (`local.bNewVisibilityLocal`) true)
      (`SceneComponent.SetHiddenInGame` _array_element_2 (not (`local.bNewVisibilityLocal`)) true)
      (`PrimitiveComponent.SetCollisionEnabled` _array_element_2 (select `bool` (`local.bNewVisibilityLocal`) :`false` "NoCollision" :`true` "QueryAndPhysics" :!type "ECollisionEnabled Enum"))))
  (return))

(fn `UserConstructionScript`)