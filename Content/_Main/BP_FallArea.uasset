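; BP_FallArea is a trigger volume that catches the player in fall areas and sends them back to the last crossroads.
; The construction script fixes the size and scale of the Box trigger and the static mesh, which is hidden at BeginPlay.
; When an actor tagged Player overlaps the Box, it plays an invalid-action sound and calls ReturnToLastCrossroadsMessage on that actor's instigator controller, which handles the return.
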(event `self.ReceiveBeginPlay`
  (bind _staticmesh (`self.StaticMesh`))
  (`SceneComponent.SetVisibility` _staticmesh false false)
  (`SceneComponent.SetHiddenInGame` _staticmesh true false))

(event `self.Box.OnComponentBeginOverlap`
  (params (OverlappedComponent :type "PrimitiveComponent Object Reference") (OtherActor :type "Actor Object Reference") (OtherComp :type "PrimitiveComponent Object Reference") (OtherBodyIndex :type Integer) (bFromSweep :type Boolean) (SweepResult :type "HitResult Structure (by ref)"))
  (if (`self.ActorHasTag` OtherActor "Player")
    (`GameplayStatics.PlaySound2D` "/Engine/VREditor/Sounds/UI/Invalid_Action.Invalid_Action" 1.5 1.0 0.0 null null)
    (message `/Game/_Main/BI_TopDownController.ReturnToLastCrossroads` (`self.GetInstigatorController` OtherActor))))

(fn `UserConstructionScript`
  (bind _box (`self.Box`))
  (`SceneComponent.SetRelativeScale3D` (`self.StaticMesh`) (10.0 10.0 2.5))
  (`BoxComponent.SetBoxExtent` _box (32.0 32.0 32.0) true)
  (`SceneComponent.SetRelativeScale3D` _box (1.5 1.5 1.5)))