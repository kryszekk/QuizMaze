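; Point-of-interest actor that the player triggers once by walking into it.
; When an actor tagged Player overlaps its box, it destroys itself and sends its ActionTag to the first player controller through a DoPOIAction message.
; If Rotate is enabled, a looping timer with a randomized start turns the static mesh in small steps instead of using Tick.
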(event `self.ReceiveBeginPlay`
  (if (`self.bRotate`)
    (`KismetSystemLibrary.Delay` (`KismetMathLibrary.RandomFloatInRange` 1.0))
    (`KismetSystemLibrary.K2_SetTimerDelegate` (delegate `CustomEvent`) 0.15 true 0.91 1.0)))

(event `CustomEvent`
  (`SceneComponent.K2_AddRelativeRotation` (`self.StaticMesh`) (struct :`Yaw` 7.5) false false))

(event `self.Box.OnComponentBeginOverlap`
  (params (OverlappedComponent :type "PrimitiveComponent Object Reference") (OtherActor :type "Actor Object Reference") (OtherComp :type "PrimitiveComponent Object Reference") (OtherBodyIndex :type Integer) (bFromSweep :type Boolean) (SweepResult :type "HitResult Structure (by ref)"))
  (if (`self.ActorHasTag` OtherActor "Player")
    (`self.K2_DestroyActor`)
    (message `/Game/_Main/BI_TopDownController.DoPOIAction` (`GameplayStatics.GetPlayerController` 0) (`self.ActionTag`))))

(fn `UserConstructionScript`)